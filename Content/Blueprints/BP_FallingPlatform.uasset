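; Falling platform that drops shortly after the custom third-person character overlaps its box, then returns and rearms.
; Activate clears a Ready flag and waits briefly before Drop enables cube physics; after the fall, Reset disables physics.
; A timeline lerps the cube from its fallen transform to StartingTransform, though BeginPlay leaves the GetWorldTransform capture unwired.
; Each state swaps the cube's material, and Ready returns when the timeline finishes.
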(event `self.ReceiveBeginPlay`
  (set `self.StartingTransform` (struct)) ; Saving the starting location\nand rotation of the cube
)

(event `self.Box.OnComponentBeginOverlap`
  (params (OverlappedComponent :type "PrimitiveComponent Object Reference") (OtherActor :type "Actor Object Reference") (OtherComp :type "PrimitiveComponent Object Reference") (OtherBodyIndex :type Integer) (bFromSweep :type Boolean) (SweepResult :type "HitResult Structure (by ref)"))
  (cast `/Game/Blueprints/BP_ThirdPersonCharacterCustom` OtherActor) ; DId the player step on the platform
  (`self.Activate`))

(event `Activate`
  (if (`self.Ready`)
    (`KismetSystemLibrary.PrintString` "1 second left")
    (set `self.Ready` false) ; The platform cannot be reactivated until\nit has been reset
    (`PrimitiveComponent.SetMaterial` (`self.Cube`) 0 "/Game/Materials/MI_PlatformActivated.MI_PlatformActivated")
    (`KismetSystemLibrary.Delay` 1.0)
    (`self.Drop`)))

(event `Drop`
  (`KismetSystemLibrary.PrintString` "Dropping!")
  (`PrimitiveComponent.SetSimulatePhysics` (`self.Cube`) true)
  (`PrimitiveComponent.SetMaterial` (`self.Cube`) 0 "/Game/Materials/MI_PlatformFalling.MI_PlatformFalling")
  (`KismetSystemLibrary.Delay` 3.0) ; Fall for 3 seconds
  (`self.Reset`))

(event `Reset`
  (`KismetSystemLibrary.PrintString` "Resetting")
  (set `self.ResetTransform` (`SceneComponent.K2_GetComponentToWorld` (`self.Cube`)))
  (`PrimitiveComponent.SetSimulatePhysics` (`self.Cube`) false)
  (`PrimitiveComponent.SetMaterial` (`self.Cube`) 0 "/Game/Materials/MI_PlatformResetting.MI_PlatformResetting")
  (bind (_direction _float) (`Timeline|GoBackToStart` :!via `PlayFromStart`)
    (:`Update`
      (bind (_returnvalue_location _returnvalue_rotation) (`KismetMathLibrary.BreakTransform` (`KismetMathLibrary.TLerp` (`self.ResetTransform`) (`self.StartingTransform`) _float)))
      (`SceneComponent.K2_SetWorldLocationAndRotation` (`self.Cube`) _returnvalue_location _returnvalue_rotation false false))
    (:`Finished`
      (set `self.Ready` true)
      (`PrimitiveComponent.SetMaterial` (`self.Cube`) 0 "/Game/Materials/MI_PlatformReady.MI_PlatformReady"))))

(fn `UserConstructionScript`)